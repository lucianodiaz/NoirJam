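; Player controller for point-and-click movement, viewed through a BP_Camera placed in the level.
; On BeginPlay it finds the first BP_Camera and sets it as the view target.
; MainAction traces under the cursor, then sends the pawn to the hit InteractableActor, or otherwise to the hit location, using simple move-to calls.
; Both move helpers also turn the control rotation toward the destination; reaching an actor triggers no interaction here.
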(event EventBeginPlay
  (bind _outactors (Actor|GetAllActorsOfClass "/Game/Core/BP_Camera.BP_Camera_C"))
  (bind _output_get (Variables|Default|SetAdventureCamera (Utilities|Array|Get(acopy) _outactors)))
  (Game|Player|SetViewTargetwithBlend _output_get 0.0 "VTBlend_Linear" 0.0 false))

(event Input|ActionEvents|InputActionMainAction
  (params (Key :type Key%20Structure :default "None"))
  (bind _hitresult (Game|Player|GetHitResultUnderCursorbyChannel "TraceTypeQuery1" true))
  (bind (_bblockinghit _binitialoverlap _time _distance _location _impactpoint _normal _impactnormal _physmat _hitactor) (Collision|BreakHitResult _hitresult))
  (:Pressed
    (bind _asinteractable_actor (Utilities|Casting|CastToInteractableActor _hitactor)
      (:then
        (CallFunction|MovetoSelectedActor _asinteractable_actor))
      (:CastFailed
        (CallFunction|MovetoSelectedLocation _location _location)))))

(fn ConstructionScript)

(fn MovetoSelectedActor
  (params (Goal :type Actor%20Object%20Reference))
  (AI|Navigation|SimpleMovetoActor self Goal)
  (Pawn|SetControlRotation (Math|Rotator|FindLookatRotation (Transformation|GetActorLocation (Pawn|GetControlledPawn)) (Transformation|GetActorLocation Goal))))

(fn MovetoSelectedLocation
  (params (Goal :type Vector%20%28by%20ref%29) (Target :type Vector%20%28by%20ref%29))
  (AI|Navigation|SimpleMovetoLocation self Goal)
  (Pawn|SetControlRotation (Math|Rotator|FindLookatRotation (Transformation|GetActorLocation (Pawn|GetControlledPawn)) Target)))